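; MainCamera is a player-possessed camera actor that keeps a camel in view.
; On BeginPlay player controller 0 possesses it.
; Every tick it rotates the whole actor to face the FocusingCamel reference.
; The mouse wheel zooms by sliding the Camera component along its local X axis in fixed steps, with no limits.
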(event EventBeginPlay
  (Pawn|Possess (Game|GetPlayerController 0) self))

(event EventTick
  (params (DeltaSeconds :type Float%20%28single-precision%29))
  ;[1 1 1] Rotates camera to focus on the camel
  (Transformation|SetActorRotation (Math|Conversions|RotationFromXVector (Math|Vector|GetUnitDirection(Vector) (Transformation|GetActorLocation) (Transformation|GetActorLocation (Variables|Default|GetFocusing%20Camel))))))

(event Input|MouseEvents|MouseWheelUp
  (params (Key :type Key%20Structure))
  (bind _camera (Variables|Default|GetCamera))
  (:Pressed
    (Transformation|SetRelativeLocation _camera (+ (Variables|/Script/Engine.SceneComponent|GetRelativeLocation _camera) "100.000000, 0, 0") false false)))

(event Input|MouseEvents|MouseWheelDown
  (params (Key :type Key%20Structure))
  (bind _camera (Variables|Default|GetCamera))
  (:Pressed
    (Transformation|SetRelativeLocation _camera (+ (Variables|/Script/Engine.SceneComponent|GetRelativeLocation _camera) "-100.000000, 0, 0") false false)))

(fn ConstructionScript)