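; A camel racer actor that runs along a chain of goal posts, timing itself until it reaches the finish.
; Tick accelerates it toward the current post and polls per-camel sprint and jump keys on player controller 0.
; Limited sprints give timed boosts, then lower the speed multiplier until timeline-driven recharges restore them.
; A timeline lifts the cube for jumps, while text renders show controller number, sprints and finish time.
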(event Custom|Pause%20Refresh
  (Timeline|Timeline_1 Stop
    (:Finished
      (if (not (>= (Variables|Default|GetSprints) (Variables|Default|GetDefaultSprints)))
        (Variables|Default|SetSprints (+ (Variables|Default|GetSprints) 1))
        (CallFunction|UpdateSpeedRed)
        (CallFunction|Refresh)))))

(event Custom|Refresh
  (Timeline|Timeline_1 PlayFromStart
    (:Finished
      (if (not (>= (Variables|Default|GetSprints) (Variables|Default|GetDefaultSprints)))
        (Variables|Default|SetSprints (+ (Variables|Default|GetSprints) 1))
        (CallFunction|UpdateSpeedRed)
        (CallFunction|Refresh)))))

(event Custom|Sprint
  (Variables|Default|SetCan%20Sprint false)
  (Variables|Default|SetSprints (- (Variables|Default|GetSprints) 1))
  (Variables|Default|SetTopSpeedPercent 1.0)
  (CallFunction|PauseRefresh)
  (Variables|Default|SetSprintBonus (Variables|Default|GetSprintSpeed))
  (Timeline|Timeline_0 PlayFromStart
    (:Finished
      (Variables|Default|SetCan%20Sprint true)
      (CallFunction|UpdateSpeedRed)
      (Variables|Default|SetSprintBonus 0.0)
      (CallFunction|Refresh))))

(event Custom|SetSprintsColor
  (Rendering|Components|TextRender|SetTextRenderColor (Variables|Default|GetTextRender1) (Math|Color|MakeColor (- 255 (* 255 (Math|Conversions|ToByte(Integer) (not (Variables|Default|GetCan%20Sprint))))) 255 255)))

(event Custom|UpdateSpeedRed
  (bind _defaultsprints (Variables|Default|GetDefaultSprints))
  (if (!= (Variables|Default|GetDefaultSprints) 0)
    (Variables|Default|SetTopSpeedPercent (- 1.0 (* (/ (Math|Conversions|ToFloat(Integer) (- _defaultsprints (Variables|Default|GetSprints))) (Math|Conversions|ToFloat(Integer) _defaultsprints)) (Variables|Default|GetPercentSpeedReduction))))))

(event Custom|Cube%20Jump
  (Variables|Default|SetisJumping true)
  (bind _height (Timeline|JumpTimeline PlayFromStart)
    (:Update
      (Transformation|SetRelativeLocation (Variables|Default|GetCube) (Math|Vector|MakeVector 0.0 0.0 (* _height (Variables|Default|GetMaxJumpHeight))) false false)
      (Variables|Default|SetIsInAir (>= (* _height (Variables|Default|GetMaxJumpHeight)) 1e+01)))
    (:Finished
      (Variables|Default|SetisJumping false))))

(event Collision|EventActorBeginOverlap
  (params (OtherActor :type Actor%20Object%20Reference))
  (if (== OtherActor (Variables|Default|GetCurrentGoal))
    (if (Variables|/Game/Blueprints/Goalpost.Goalpost_C|GetisGoal? (Variables|Default|GetCurrentGoal))
      (Variables|Default|SetisRacing false)
      (Rendering|Components|TextRender|SetText (Variables|Default|GetTextRender1) (Utilities|Text|ToText(Float) (Variables|Default|GetFinishtime) "HalfToEven"))
      (else
        (Variables|Default|SetCurrentGoal (Variables|/Game/Blueprints/Goalpost.Goalpost_C|GetnextPost (Variables|Default|GetCurrentGoal)))))))

(event EventTick
  (params (DeltaSeconds :type Float%20%28single-precision%29))
  (if (Variables|Default|GetisRacing)
    (Rendering|Components|TextRender|SetText (Variables|Default|GetTextRender1) (Utilities|Text|ToText(Integer) (Variables|Default|GetSprints)))
    (CallFunction|SetSprintsColor)
    (Variables|Default|SetFinishtime (+ (Variables|Default|GetFinishtime) DeltaSeconds))
    (Transformation|SetActorLocation (+ (Transformation|GetActorLocation) (Math|Vector|RotateVector (Math|Vector|MakeVector (* DeltaSeconds (* (+ (Variables|Default|GetCurrent%20Speed) (Variables|Default|GetSprintBonus)) (Variables|Default|GetTopSpeedPercent)) 1e+02) 0.0 0.0) (Math|Conversions|RotationFromXVector (Math|Vector|GetUnitDirection(Vector) (Transformation|GetActorLocation) (Transformation|GetActorLocation (Variables|Default|GetCurrentGoal)))))) false false)
    (if (>= (Variables|Default|GetTopSpeed) (+ (Variables|Default|GetCurrent%20Speed) (Variables|Default|GetAcceleration)))
      (Variables|Default|SetCurrent%20Speed (+ (Variables|Default|GetCurrent%20Speed) (Variables|Default|GetAcceleration))))
    (if (Math|Boolean|ANDBoolean (Game|Player|IsInputKeyDown (Game|GetPlayerController 0) (Variables|Default|GetSprintKey)) (Variables|Default|GetCan%20Sprint) (> (Variables|Default|GetSprints) 0))
      (CallFunction|Sprint))
    (if (and (Game|Player|IsInputKeyDown (Game|GetPlayerController 0) (Variables|Default|GetJumpKey)) (not (Variables|Default|GetisJumping)))
      (CallFunction|CubeJump))))

(event EventBeginPlay
  (Variables|Default|SetSprints (Variables|Default|GetDefaultSprints))
  (bind _output_get (Variables|Default|SetNumber (Utilities|String|ToString(Integer) (Variables|Default|GetController))))
  (Rendering|Components|TextRender|SetText (Variables|Default|GetTextRender) (Utilities|Text|ToText(String) _output_get))
  (Variables|Default|SetTopSpeedPercent 1.0))

(fn ConstructionScript)